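; LD_Controller is a player controller that turns the controlled ThirdPersonCharacter to face the mouse cursor while it is aiming.
; Each tick it deprojects the cursor into a world ray and intersects it with a horizontal plane at the pawn's location, using a line-plane macro.
; When a point is found and Aiming is set, the pawn's rotation snaps to look at that point, without needing a collision trace.
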(event EventTick
  (params (DeltaSeconds :type Float%20%28single-precision%29))
  (bind (_worldlocation _worlddirection) (Game|Player|ConvertMouseLocationToWorldSpace))
  (bind _returnvalue (Pawn|GetControlledPawn))
  (bind _returnvalue_2 (Transformation|GetActorLocation _returnvalue))
  (bind (_intersectionpoint _pointfound) (Utilities|NewMacro0 _worldlocation _worlddirection 5e+05 _returnvalue_2 "0,0,1.000000"))
  (if _pointfound
    (bind _asthird_person_character (Utilities|Casting|CastToThirdPersonCharacter (Pawn|GetControlledPawn)))
    (if (Variables|/Game/Blueprints/ThirdPersonCharacter.ThirdPersonCharacter_C|GetAiming _asthird_person_character)
      (Transformation|SetActorRotation (Pawn|GetControlledPawn) (Math|Rotator|FindLookatRotation _returnvalue_2 _intersectionpoint)))))

(fn ConstructionScript)