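; Bonfire actor where the player places an egg, then lights it with logs to hatch a Phoenix.
; Overlap gives the ThirdPersonCharacter a bonfire reference and allows lighting based on its held resource: egg first, logs afterwards.
; LitBonfire either spawns the egg or breaks it and refills FireLevel, spawning the Phoenix only on first ignition.
; That ignition also starts a looping timer that steadily lowers FireLevel and dims the point light.
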(event Custom|LitBonfire
  (if (Variables|Default|GetHasPhoenix)
    (Default|Break (Variables|Default|GetEggRef))
    (Variables|Default|SetFireLevel 6e+04)
    (if (Variables|Default|GetFirstIgnition)
      (Utilities|Time|SetTimerbyEvent (delegate Custom|FireDegrading) 1.0 true)
      (Variables|Default|SetFirstIgnition false)
      (Rendering|Components|Light|SetIntensity (Variables|Default|GetPointLight) (Variables|Default|GetFireLevel))
      (Game|SpawnActorfromClass "/Game/Blueprints/Characters/Phoenix.Phoenix_C" (Transformation|GetWorldTransform (Variables|Default|GetPointLight)) "Undefined" 0 0))
    (else
      (bind _returnvalue (Game|SpawnActorfromClass "/Game/Blueprints/World/BonfireEgg.BonfireEgg_C" (Transformation|GetWorldTransform (Variables|Default|GetPointLight)) "Undefined" 0 0))
      (Variables|Default|SetEggRef _returnvalue)
      (Variables|Default|SetHasPhoenix true))))

(event Custom|FireDegrading
  (bind _output_get (Variables|Default|SetFireLevel (- (Variables|Default|GetFireLevel) 1e+03)))
  (Rendering|Components|Light|SetIntensity (Variables|Default|GetPointLight) _output_get))

(event Collision|EventActorBeginOverlap
  (params (OtherActor :type Actor%20Object%20Reference))
  (bind _asthird_person_character (Utilities|Casting|CastToThirdPersonCharacter OtherActor))
  (Variables|/Game/Blueprints/ThirdPersonCharacter.ThirdPersonCharacter_C|SetBonfireRef _asthird_person_character self)
  (bind _output_get (Variables|Default|SetPlayerRef _asthird_person_character))
  (if (Utilities|IsValid (Variables|/Game/Blueprints/ThirdPersonCharacter.ThirdPersonCharacter_C|GetResource _output_get))
    (if (Variables|Default|GetHasPhoenix)
      (Utilities|Casting|CastToBP_LogsClass (Utilities|GetClass (Variables|/Game/Blueprints/ThirdPersonCharacter.ThirdPersonCharacter_C|GetResource _output_get)))
      (else
        (Utilities|Casting|CastToBP_EggClass (Utilities|GetClass (Variables|/Game/Blueprints/ThirdPersonCharacter.ThirdPersonCharacter_C|GetResource _output_get)))))
    (Variables|/Game/Blueprints/ThirdPersonCharacter.ThirdPersonCharacter_C|SetCanLightBonfire (Variables|Default|GetPlayerRef) true)))

(event Collision|EventActorEndOverlap
  (params (OtherActor :type Actor%20Object%20Reference))
  (bind _asthird_person_character (Utilities|Casting|CastToThirdPersonCharacter OtherActor))
  (Variables|/Game/Blueprints/ThirdPersonCharacter.ThirdPersonCharacter_C|SetBonfireRef _asthird_person_character 0)
  (Variables|/Game/Blueprints/ThirdPersonCharacter.ThirdPersonCharacter_C|SetCanLightBonfire _asthird_person_character false)
  (Variables|Default|SetPlayerRef 0))

(fn ConstructionScript)