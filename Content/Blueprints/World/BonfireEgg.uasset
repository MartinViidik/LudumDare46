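; BonfireEgg is a world egg actor with speech bubbles that cracks open when its Break event is called.
; On BeginPlay it plays a 2D UI pop sound and hides the bottom and top shell pieces.
; Break swaps the whole egg and both bubbles for those pieces.
; It then enables physics and gravity on the destructible top shell and shatters it with high radius damage and impulse from the actor's location.
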(event Custom|Break
  (Rendering|SetVisibility (Variables|Default|GetSpeechBubble) false false)
  (Rendering|SetVisibility (Variables|Default|GetSpeechBubble1) false false)
  (Rendering|SetVisibility (Variables|Default|GetEggBottom) true false)
  (Rendering|SetVisibility (Variables|Default|GetTopEggShell_DM) true false)
  (Rendering|SetVisibility (Variables|Default|GetEggFull) false false)
  (Physics|SetEnableGravity (Variables|Default|GetTopEggShell_DM) true)
  (Physics|SetSimulatePhysics (Variables|Default|GetTopEggShell_DM) true)
  (Class|DestructibleComponent|ApplyRadiusDamage (Variables|Default|GetTopEggShell_DM) 1e+04 (Transformation|GetActorLocation) 0.0 1e+04 false))

(event EventBeginPlay
  (Class|FMODBlueprintStatics|PlayEvent2D "/Game/FMOD/Events/sfx_ui_pops.sfx_ui_pops")
  (Rendering|SetVisibility (Variables|Default|GetEggBottom) false false)
  (Rendering|SetVisibility (Variables|Default|GetTopEggShell_DM) false false))

(fn ConstructionScript)