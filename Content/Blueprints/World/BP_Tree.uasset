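; BP_Tree is a choppable tree actor that falls over and spawns loot.
; On overlap begin and end it sets or clears the ThirdPersonCharacter's TreeRef.
; CutDown plays the Treefall timeline, whose TreeRotation track pitches and offsets Trunk1 while enabling physics each update.
; When the timeline finishes, physics is turned off and the Loot class spawns at the actor's location.
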(event Custom|CutDown
  (bind _trunk1 (Variables|Default|GetTrunk1))
  (bind _treerotation (Timeline|Treefall Play)
    (:Update
      (Transformation|SetWorldLocationAndRotation _trunk1 (- (Transformation|GetWorldLocation (Variables|Default|GetTrunk1)) (Math|Vector|MakeVector (/ _treerotation 5e+01) 0.0 (/ _treerotation 5e+01))) (Math|Rotator|MakeRotator 0.0 _treerotation 0.0) false false)
      (Physics|SetSimulatePhysics _trunk1 true))
    (:Finished
      (Physics|SetSimulatePhysics (Variables|Default|GetTrunk1) false)
      (Game|SpawnActorfromClass (Variables|Default|GetLoot) (Math|Conversions|ToTransform(Vector) (Transformation|GetActorLocation)) "Undefined" 0 0))))

(event Collision|EventActorBeginOverlap
  (params (OtherActor :type Actor%20Object%20Reference))
  (bind _asthird_person_character (Utilities|Casting|CastToThirdPersonCharacter OtherActor))
  (Variables|/Game/Blueprints/ThirdPersonCharacter.ThirdPersonCharacter_C|SetTreeRef _asthird_person_character self))

(event Collision|EventActorEndOverlap
  (params (OtherActor :type Actor%20Object%20Reference))
  (bind _asthird_person_character (Utilities|Casting|CastToThirdPersonCharacter OtherActor))
  (Variables|/Game/Blueprints/ThirdPersonCharacter.ThirdPersonCharacter_C|SetTreeRef _asthird_person_character 0))

(fn ConstructionScript)