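; BP_Item is a pickup actor that registers itself on the overlapping ThirdPersonCharacter as either a ground resource or a ground item, depending on its ItemType.
; On pickup, a resource snaps to the player's Egg component every few milliseconds via a looping timer until ClearEvents stops it.
; Other items drop below their position and become the player's Item, and ReturnItem raises them back up.
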(event Custom|PickupItem
  (bind _returnvalue (Game|GetPlayerCharacter 0))
  (if (Utilities|Enum|Equal(Enum) (Variables|Default|GetItemType) "NewEnumerator3")
    (bind _asthird_person_character (Utilities|Casting|CastToThirdPersonCharacter _returnvalue))
    (Variables|/Game/Blueprints/ThirdPersonCharacter.ThirdPersonCharacter_C|SetResource _asthird_person_character self)
    (Development|PrintString "Hello")
    (Variables|Default|SetPlayerRef _asthird_person_character)
    (bind _returnvalue_2 (Utilities|Time|SetTimerbyEvent (delegate Custom|SetLocation) 0.005 true))
    (else
      (Transformation|SetActorLocation (- (Transformation|GetActorLocation) "0, 0,110.000000") false false)
      (bind _asthird_person_character_2 (Utilities|Casting|CastToThirdPersonCharacter _returnvalue))
      (Variables|/Game/Blueprints/ThirdPersonCharacter.ThirdPersonCharacter_C|SetItem _asthird_person_character_2 self))))

(event Custom|SetLocation
  (bind _playerref (Variables|Default|GetPlayerRef))
  (bind _egg (Variables|/Game/Blueprints/ThirdPersonCharacter.ThirdPersonCharacter_C|GetEgg _playerref))
  (Transformation|SetActorLocation (Transformation|GetWorldLocation _egg) false false)
  (Transformation|SetActorRotation (Transformation|GetWorldRotation _egg)))

(event Custom|ReturnItem
  (Development|PrintString "Returning")
  (Transformation|SetActorLocation (+ (Transformation|GetActorLocation) "0, 0,110.000000") false false)
  (Variables|Default|SetPlayerRef 0))

(event Custom|ClearEvents
  (Utilities|Time|ClearandInvalidateTimerbyHandle (stale Custom|PickupItem _returnvalue_2))
  (Variables|Default|SetPlayerRef 0)
  (Transformation|SetActorRotation "0, 0, 0"))

(event EventBeginPlay)

(event Collision|EventActorBeginOverlap
  (params (OtherActor :type Actor%20Object%20Reference))
  (bind _self self)
  (if (not (Utilities|IsValid (Variables|Default|GetPlayerRef)))
    (if (Utilities|Enum|Equal(Enum) (Variables|Default|GetItemType) "NewEnumerator3")
      (bind _asthird_person_character (Utilities|Casting|CastToThirdPersonCharacter OtherActor))
      (Variables|/Game/Blueprints/ThirdPersonCharacter.ThirdPersonCharacter_C|SetGroundResource _asthird_person_character _self)
      (else
        (bind _asthird_person_character_2 (Utilities|Casting|CastToThirdPersonCharacter OtherActor))
        (Variables|/Game/Blueprints/ThirdPersonCharacter.ThirdPersonCharacter_C|SetGroundItem _asthird_person_character_2 _self)))))

(event Collision|EventActorEndOverlap
  (params (OtherActor :type Actor%20Object%20Reference))
  (if (Utilities|Enum|Equal(Enum) (Variables|Default|GetItemType) "NewEnumerator3")
    (bind _asthird_person_character (Utilities|Casting|CastToThirdPersonCharacter OtherActor))
    (Variables|/Game/Blueprints/ThirdPersonCharacter.ThirdPersonCharacter_C|SetGroundResource _asthird_person_character 0)
    (else
      (bind _asthird_person_character_2 (Utilities|Casting|CastToThirdPersonCharacter OtherActor))
      (Variables|/Game/Blueprints/ThirdPersonCharacter.ThirdPersonCharacter_C|SetGroundItem _asthird_person_character_2 0))))

(fn ConstructionScript)