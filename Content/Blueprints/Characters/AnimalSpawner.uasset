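; AnimalSpawner creates an Animal at its own location and replaces it once it is gone.
; SpawnAnimal stores the new actor, starts a looping validity timer and plays a timeline that scales the animal's capsule uniformly.
; When CheckAnimal finds the reference invalid, it clears the timer and calls SpawnAnimal again, which starts a fresh one.
; Nothing in this graph calls the first spawn.
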(event Custom|SpawnAnimal
  (bind _returnvalue (Game|SpawnActorfromClass (Variables|Default|GetAnimal) (Math|Conversions|ToTransform(Vector) (Transformation|GetActorLocation)) "AlwaysSpawn" 0 0))
  (Variables|Default|SetAnimalRef _returnvalue)
  (bind _returnvalue_2 (Utilities|Time|SetTimerbyEvent (delegate Custom|CheckAnimal) 9.0 true))
  (bind _newtrack_0 (Timeline|Timeline_0 Play)
    (:Update
      (Transformation|SetWorldScale3D (Variables|/Script/Engine.Character|GetCapsuleComponent (Variables|Default|GetAnimalRef)) (Math|Vector|MakeVector _newtrack_0 _newtrack_0 _newtrack_0)))))

(event Custom|CheckAnimal
  (if (not (Utilities|IsValid (Variables|Default|GetAnimalRef)))
    (Utilities|Time|ClearandInvalidateTimerbyHandle (stale Custom|SpawnAnimal _returnvalue_2))
    (CallFunction|SpawnAnimal)))

(fn ConstructionScript)