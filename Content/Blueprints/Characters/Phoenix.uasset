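; Phoenix is a character that demands a random food type and checks what the player brings on overlap.
; On BeginPlay it stores the player's ThirdPersonCharacter and picks a demand from FoodTypes, swapping one enum value for another fallback.
; When the player overlaps holding a valid Resource, a matching FoodType triggers a new demand, while a mismatch keeps the current one.
; All feedback is printed strings, and the held resource is left untouched.
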(event Custom|DemandItem
  (bind _output_get (Variables|Default|SetFoodDemand (Utilities|Array|Get(acopy) (Variables|Default|GetFoodTypes) (Math|Random|RandomIntegerinRange 0 (Utilities|Array|Length (Variables|Default|GetFoodTypes))))))
  (if (Utilities|Enum|Equal(Enum) _output_get "NewEnumerator2")
    (Development|PrintString "Hello")
    (bind _output_get_2 (Variables|Default|SetFoodDemand "NewEnumerator0"))
    (Development|PrintString (Utilities|String|EnumtoString _output_get_2))
    (else
      (Development|PrintString (Utilities|String|EnumtoString _output_get)))))

(event EventBeginPlay
  (bind _asthird_person_character (Utilities|Casting|CastToThirdPersonCharacter (Game|GetPlayerCharacter 0)))
  (Variables|Default|SetPlayerRef _asthird_person_character)
  (CallFunction|DemandItem))

(event Collision|EventActorBeginOverlap
  (params (OtherActor :type Actor%20Object%20Reference))
  (bind _playerref (Variables|Default|GetPlayerRef))
  (bind _resource (Variables|/Game/Blueprints/ThirdPersonCharacter.ThirdPersonCharacter_C|GetResource _playerref))
  (if (== OtherActor (Variables|Default|GetPlayerRef))
    (if (Utilities|IsValid _resource)
      (if (Utilities|Enum|Equal(Enum) (Variables|Default|GetFoodDemand) (Variables|/Game/Blueprints/Items/BP_Item.BP_Item_C|GetFoodType _resource))
        (Development|PrintString "Yay")
        (CallFunction|DemandItem)
        (else
          (Development|PrintString "Nay"))))))

(fn ConstructionScript)